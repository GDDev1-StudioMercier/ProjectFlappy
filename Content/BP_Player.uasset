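; Player Blueprint for a physics-driven, flap-style character that registers its Enhanced Input mapping on BeginPlay.
; The first jump enables mesh physics and plays a timeline that slides the camera along its relative Y, paced by SpeedCamera.
; Every jump zeroes the velocity before applying a fixed upward impulse, so each hop is consistent.
; Tick maps vertical velocity to a clamped mesh pitch, tilting it as it rises and falls.
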(event `self.ReceiveBeginPlay`
  (bind _asplayer_controller (cast `PlayerController` (`self.GetController`)))
  (`EnhancedInputSubsystemInterface.AddMappingContext` (pcsubsystem `EnhancedInputLocalPlayerSubsystem` _asplayer_controller) "/Game/Inputs/IMC_Player.IMC_Player" 0 (struct))
  (`TimelineComponent.SetPlayRate` (`self.LerpCam`) (/ 1.0 (`self.SpeedCamera`))))

(event `self.ReceiveTick`
  (params (DeltaSeconds :type "Float (single-precision)"))
  (bind _skeletalmesh (`self.SkeletalMesh`))
  (bind (_returnvalue_x _returnvalue_y _returnvalue_z) (`KismetMathLibrary.BreakVector` (`SceneComponent.GetComponentVelocity` _skeletalmesh)))
  (`SceneComponent.K2_SetWorldRotation` _skeletalmesh (`KismetMathLibrary.MakeRotator` 0.0 (`KismetMathLibrary.MapRangeClamped` _returnvalue_z -900.0 900.0 -45.0 45.0)) false true))

(event `EnhancedInput|/Game/Inputs/Actions/IA_Jump`
  (params (ActionValue :type Boolean) (ElapsedSeconds :type "Float (double-precision)") (TriggeredSeconds :type "Float (double-precision)") (InputAction :type "InputAction Object Reference" :default "/Game/Inputs/Actions/IA_Jump.IA_Jump"))
  (bind _skeletalmesh (`self.SkeletalMesh`))
  (:`Started`
    (`|ExecutionSequence`
      (:`then_0`
        (`/Engine/EditorBlueprintResources/StandardMacros.DoOnce` false
          (:`Completed`
            (`PrimitiveComponent.SetSimulatePhysics` (`self.SkeletalMesh`) true)
            (bind (_direction _newtrack_0) (`Timeline|LerpCam`)
              (:`Update`
                (`SceneComponent.K2_SetRelativeLocation` (`self.Camera`) (`KismetMathLibrary.MakeVector` 0.0 (`KismetMathLibrary.Lerp` 200.0 600.0 _newtrack_0)) false false))))))
      (:`then_1`
        (`PrimitiveComponent.SetPhysicsLinearVelocity` _skeletalmesh (0.0 0.0 0.0) false "None")
        (`PrimitiveComponent.AddImpulse` _skeletalmesh (0.0 0.0 1000.0) "None" true)))))

(fn `UserConstructionScript`)